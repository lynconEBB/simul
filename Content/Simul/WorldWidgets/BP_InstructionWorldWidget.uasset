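; An instruction panel Blueprint that displays header, body and footer text with optional image and video through a world widget component.
; On widget init, it caches the WBP_Instructions widget and applies its visibility flags, column fills, texts and image sizing from its variables.
; On BeginPlay, if video is enabled, it opens a looping media source and fits the media texture into that cached widget using the track dimensions.
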(event `self.WidgetComponent.OnInitWidget`
  (bind _output (`|ConvertAsset` (`self.Widget`)))
  (bind _gridpanel_76 (`/Game/Simul/GUI/Components/WBP_Instructions.GridPanel_76` _output))
  (bind _aswbp_instructions (cast `/Game/Simul/GUI/Components/WBP_Instructions` (`WidgetComponent.GetWidget` (`self.WidgetComponent`))))
  (set `self.Widget` (`|ConvertAsset` _aswbp_instructions))
  (`|ExecutionSequence`
    (:`then_0`
      (set `/Game/Simul/GUI/Components/WBP_Instructions.bDisplayFooter` (`self.bShowFooter`) _output)
      (set `/Game/Simul/GUI/Components/WBP_Instructions.bDisplayHeader` (`self.bShowHeader`) _output)
      (set `/Game/Simul/GUI/Components/WBP_Instructions.bDisplayVideo` (`self.bShowVideo`) _output)
      (set `/Game/Simul/GUI/Components/WBP_Instructions.bDisplayImage` (`self.bShowImage`) _output)
      (`GridPanel.SetColumnFill` _gridpanel_76 0 (`self.TextFill`))
      (`GridPanel.SetColumnFill` _gridpanel_76 1 (`self.VideoImageFill`)))
    (:`then_1`
      (`TextBlock.SetText` (`/Game/Simul/GUI/Components/WBP_Instructions.HeaderText` (`|ConvertAsset` (`self.Widget`))) (`KismetTextLibrary.Conv_StringToText` (`self.HeaderText`)))
      (`TextBlock.SetText` (`/Game/Simul/GUI/Components/WBP_Instructions.FooterText` (`|ConvertAsset` (`self.Widget`))) (`KismetTextLibrary.Conv_StringToText` (`self.FooterText`)))
      (`TextBlock.SetText` (`/Game/Simul/GUI/Components/WBP_Instructions.ContentText` (`|ConvertAsset` (`self.Widget`))) (`KismetTextLibrary.Conv_StringToText` (`self.ContentText`))))
    (:`then_2`
      (if (`self.bShowImage`)
        (`Image.SetBrushFromTexture` (`/Game/Simul/GUI/Components/WBP_Instructions.ContentImage` (`|ConvertAsset` (`self.Widget`))) (`self.Image`) true)
        (`HorizontalBoxSlot.SetSize` (`WidgetLayoutLibrary.SlotAsHorizontalBoxSlot` (`/Game/Simul/GUI/Components/WBP_Instructions.ImageOverlay` (`|ConvertAsset` (`self.Widget`)))) (make `SlateChildSize` (`self.ImageFill`)))
        (if (> (`self.ImageMaxWidth`) 0.0)
          (`SizeBox.SetMaxDesiredWidth` (`/Game/Simul/GUI/Components/WBP_Instructions.ImageSizeBox` (`|ConvertAsset` (`self.Widget`))) (`self.ImageMaxWidth`)))))))

(event `self.ReceiveBeginPlay`
  (if (`self.bShowVideo`)
    (bind _videomediaplayer (`self.VideoMediaPlayer`)
      (:`then`
        (`MediaPlayer.OpenSourceLatent` _videomediaplayer (`self.VideoMediaSource`) (make `MediaPlayerOptions` (struct :`Caption` -1 :`Metadata` -1 :`Script` -1 :`Subtitle` -1 :`Text` -1) "+00000000.00:00:00.000000000" "Enabled" "Enabled"))
        (`Image.SetBrushResourceObject` (`/Game/Simul/GUI/Components/WBP_Instructions.ContentVideo` (`|ConvertAsset` (`self.Widget`))) (`self.VideoMediaTexture`))
        (`Image.SetBrushSize` (`/Game/Simul/GUI/Components/WBP_Instructions.ContentVideo` (`|ConvertAsset` (`self.Widget`))) (`KismetMathLibrary.Conv_IntPointToVector2D` (`MediaPlayer.GetVideoTrackDimensions` (`self.VideoMediaPlayer`) -1 -1)))
        (`HorizontalBoxSlot.SetSize` (`WidgetLayoutLibrary.SlotAsHorizontalBoxSlot` (`/Game/Simul/GUI/Components/WBP_Instructions.VideoOverlay` (`|ConvertAsset` (`self.Widget`)))) (make `SlateChildSize` (`self.VideoFill`)))
        (if (> (`self.VideoMaxWidth`) 0.0)
          (`SizeBox.SetMaxDesiredWidth` (`/Game/Simul/GUI/Components/WBP_Instructions.VideoSizeBox` (`|ConvertAsset` (`self.Widget`))) (`self.VideoMaxWidth`))))
      (:`else`))))

(fn `UserConstructionScript`)