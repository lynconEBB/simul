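; BP_GrippableCube is a grippable, colored cube that reports slot placement to the simulation.
; Its Slottable component's slotted and unslotted events switch the cube's State on or off in the SimulationSubsystem.
; Overlapping a SlotComponent that lacks the mesh's first component tag throws the cube's Mistake through the same subsystem.
; The construction script applies the Color variable through a dynamic material instance.
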(event `self.Slottable.OnSlotted`
  (params (WorldTransform :type "Transform Structure") (SlotComponent :type "SlotComponent Object Reference"))
  (`SimulationSubsystem.UpdateState` (subsystem `SimulationSubsystem`) (`self.State`) true))

(event `self.Slottable.OnUnslotted`
  (params (SlotComponent :type "SlotComponent Object Reference"))
  (`SimulationSubsystem.UpdateState` (subsystem `SimulationSubsystem`) (`self.State`) false))

(event `self.GrippableStaticMesh.OnComponentBeginOverlap`
  (params (OverlappedComponent :type "PrimitiveComponent Object Reference") (OtherActor :type "Actor Object Reference") (OtherComp :type "PrimitiveComponent Object Reference") (OtherBodyIndex :type Integer) (bFromSweep :type Boolean) (SweepResult :type "HitResult Structure (by ref)"))
  (bind _asslot_component (cast `SlotComponent` OtherComp))
  (if (not (`ActorComponent.ComponentHasTag` _asslot_component (`|GetArrayItem` (`ActorComponent.ComponentTags` (`self.GrippableStaticMesh`)))))
    (`SimulationSubsystem.ThrowMistake` (subsystem `SimulationSubsystem`) (`self.Mistake`))))

(fn `UserConstructionScript`
  (bind _returnvalue (`PrimitiveComponent.CreateDynamicMaterialInstance` (`self.GrippableStaticMesh`) 0 "/Game/Simul/Maps/SimulationMap/M_Simple.M_Simple" "None"))
  (`MaterialInstanceDynamic.SetVectorParameterValue` _returnvalue "Color" (`self.Color`)))