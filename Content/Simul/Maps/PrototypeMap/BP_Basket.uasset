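; BP_Basket is a sorting basket for the simulation that checks which grippable objects are placed inside it.
; A Box overlap counts GrippableStaticMeshActors carrying TagToVerify, incrementing on entry and decrementing on exit.
; The SimulationSubsystem state is activated when the count reaches TargetCount and deactivated when it falls below.
; An entering grippable without the tag throws a WrongBasket mistake from DT_BasketMistakes.
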(event `self.Box.OnComponentBeginOverlap`
  (params (OverlappedComponent :type "PrimitiveComponent Object Reference") (OtherActor :type "Actor Object Reference") (OtherComp :type "PrimitiveComponent Object Reference") (OtherBodyIndex :type Integer) (bFromSweep :type Boolean) (SweepResult :type "HitResult Structure (by ref)"))
  (bind _asgrippable_static_mesh_actor (cast `GrippableStaticMeshActor` OtherActor))
  (if (`self.ActorHasTag` _asgrippable_static_mesh_actor (`self.TagToVerify`))
    (bind _result (`/Engine/EditorBlueprintResources/StandardMacros.IncrementInt` (`self.Count`))
      (:`  `
        (if (>= _result (`self.TargetCount`))
          (`SimulationSubsystem.UpdateState` (subsystem `SimulationSubsystem`) (`self.State`) true))))
    (else
      (`SimulationSubsystem.ThrowMistake` (subsystem `SimulationSubsystem`) (make `DataTableRowHandle` "/Game/Simul/Maps/PrototypeMap/DT_BasketMistakes.DT_BasketMistakes" "WrongBasket")))))

(event `self.Box.OnComponentEndOverlap`
  (params (OverlappedComponent :type "PrimitiveComponent Object Reference") (OtherActor :type "Actor Object Reference") (OtherComp :type "PrimitiveComponent Object Reference") (OtherBodyIndex :type Integer))
  (bind _asgrippable_static_mesh_actor (cast `GrippableStaticMeshActor` OtherActor))
  (if (`self.ActorHasTag` _asgrippable_static_mesh_actor (`self.TagToVerify`))
    (bind _result (`/Engine/EditorBlueprintResources/StandardMacros.DecrementInt` (`self.Count`))
      (:`  `
        (if (< _result (`self.TargetCount`))
          (`SimulationSubsystem.UpdateState` (subsystem `SimulationSubsystem`) (`self.State`) false))))))

(fn `UserConstructionScript`)